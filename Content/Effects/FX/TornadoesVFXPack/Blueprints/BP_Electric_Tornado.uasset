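; Electric tornado effect actor from a tornado VFX pack, built from Tornado and Ground components plus two electric arc effects.
; The construction script scales Tornado and Ground from Thickness for width and a divided-down Height for vertical size.
; Each tick, a set Stopeffect flag deactivates both arc effects, with no path to reactivate them and no change to the tornado itself.
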(event EventBeginPlay
  (|CallParentFunction) ; This node is disabled and will not be called.\nDrag off pins to build functionality.
)

(event Collision|EventActorBeginOverlap
  (params (OtherActor :type Actor%20Object%20Reference)))

(event EventTick
  (params (DeltaSeconds :type Float%20%28single-precision%29))
  (|CallParentFunction DeltaSeconds)
  (if (Variables|Default|GetbStopeffect?)
    (Components|Activation|Deactivate (Variables|Default|GetElectricArcs))
    (Components|Activation|Deactivate (Variables|Default|GetElectricArcs_02))))

(fn ConstructionScript
  (bind _height (Variables|Default|GetHeight))
  (bind _thickness (Variables|Default|GetThickness))
  (bind _returnvalue (/ _height 6.0))
  (bind _returnvalue_2 (Math|Vector|MakeVector _thickness _thickness _returnvalue))
  (|CallParentFunction)
  (Transformation|SetWorldScale3D (Variables|Default|GetTornado) _returnvalue_2)
  (Transformation|SetWorldScale3D (Variables|Default|GetGround) _returnvalue_2))