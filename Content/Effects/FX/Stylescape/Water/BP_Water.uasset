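; Stylized water actor that renders a configurable water plane with an underwater post-process effect.
; The construction script assigns the water material, pushes foam, wave and refraction parameters to it, scales the actor, and configures the post-process underwater material and blending.
; When another actor begins overlapping it, the plane's doubled world location is written to the "Water Height" parameter in the MP_Water collection.
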(event EventBeginPlay)

(event Collision|EventActorBeginOverlap
  (params (OtherActor :type Actor%20Object%20Reference))
  (Rendering|Material|SetVectorParameterValue "/Game/Effects/FX/Stylescape/Materials/Functions/MP_Water.MP_Water" "Water Height" (Math|Conversions|ToLinearColor(Vector) (* (Transformation|GetWorldLocation (Variables|Default|GetWaterPlane)) 2.0)) :!class /Script/Engine.KismetMaterialLibrary))

(event EventTick
  (params (DeltaSeconds :type Float%20%28single-precision%29)))

(fn ConstructionScript
  (bind _waterplane (Variables|Default|GetWaterPlane))
  (Rendering|Material|SetMaterial (Variables|Default|GetWaterPlane) 0 (Variables|Default|GetWaterMaterial))
  (Rendering|Material|SetScalarParameterValueonMaterials _waterplane "Foam Scale" (Variables|Default|GetFoam%20Scale))
  (Rendering|Material|SetScalarParameterValueonMaterials _waterplane "Foam Speed" (Variables|Default|GetFoam%20Speed))
  (Rendering|Material|SetScalarParameterValueonMaterials _waterplane "Foam Fade Distance" (Variables|Default|GetFoam%20Distance))
  (Rendering|Material|SetScalarParameterValueonMaterials _waterplane "Wave1 Scale" (Variables|Default|GetWave1%20Scale))
  (Rendering|Material|SetScalarParameterValueonMaterials _waterplane "Wave2 Scale" (Variables|Default|GetWave2%20Scale))
  (Rendering|Material|SetScalarParameterValueonMaterials _waterplane "Wave1 Speed" (Variables|Default|GetWave1%20Speed))
  (Rendering|Material|SetScalarParameterValueonMaterials _waterplane "Wave2 Speed" (Variables|Default|GetWave2%20Speed))
  (Rendering|Material|SetScalarParameterValueonMaterials _waterplane "Refraction Scale" (Variables|Default|GetRefraction%20Scale))
  (Rendering|Material|SetScalarParameterValueonMaterials _waterplane "Refraction Speed" (Variables|Default|GetRefraction%20Speed))
  (Transformation|SetActorScale3D (Variables|Default|GetOceanScale))
  (bind _output_get (Variables|Default|SetPostProcess (Variables|Default|GetPostProcess)))
  (Variables|/Script/Engine.PostProcessComponent|SetSettings _output_get (Utilities|Struct|MakePostProcessSettings (Variables|Default|GetUnderwaterMaterial)))
  (Variables|/Script/Engine.PostProcessComponent|SetBlendRadius _output_get (Variables|Default|GetUnderwaterBlendRadius))
  (Variables|/Script/Engine.PostProcessComponent|SetBlendWeight _output_get (Variables|Default|GetUnderwaterBlendWeight)))