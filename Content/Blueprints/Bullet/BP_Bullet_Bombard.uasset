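; BP_Bullet_Bombard is a bombard projectile that flies to a location and deals area damage to enemies.
; MakeBezierPoints defines a high five-point arc, while Tick calls FlyToLocation and explodes the bullet once its lifetime exceeds Time.
; Any actor overlap also triggers Explode, which sphere-traces around the bullet, calls AttackSingleEnemy on BP_BaseEnemy hits, spawns smoke and destroys itself.
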(event Custom|Explode
  (bind _returnvalue (Transformation|GetActorLocation))
  (Utilities|FlowControl|Sequence
    (:then_0
      (bind _outhits (Collision|MultiSphereTraceForObjects _returnvalue _returnvalue 2e+02 (Utilities|Array|MakeArray "ObjectTypeQuery7") false 0 "None"))
      (for _array_element _outhits
        (bind _asbp_base_enemy (Utilities|Casting|CastToBP_BaseEnemy (.HitActor (Collision|BreakHitResult _array_element))))
        (CallFunction|AttackSingleEnemy _asbp_base_enemy)))
    (:then_1
      (Effects|SpawnEmitteratLocation "/Game/Effects/PS_Smoke.PS_Smoke" (Transformation|GetActorLocation)))
    (:then_2
      (Actor|DestroyActor))))

(event EventBeginPlay
  (|CallParentFunction) ; This node is disabled and will not be called.\nDrag off pins to build functionality.
)

(event Collision|EventActorBeginOverlap
  (params (OtherActor :type Actor%20Object%20Reference))
  (CallFunction|Explode))

(event EventTick
  (params (DeltaSeconds :type Float%20%28single-precision%29))
  (|CallParentFunction DeltaSeconds)
  (Utilities|FlowControl|Sequence
    (:then_0
      (CallFunction|FlytoLocation))
    (:then_1
      (if (> (Actor|GetGameTimeSinceCreation) (Variables|Default|GetTime))
        (CallFunction|Explode)))))

(fn ConstructionScript
  (|CallParentFunction))

(fn MakeBezierPoints
  (params (Start :type Vector :default "0, 0, 0") (End :type Vector :default "0, 0, 0"))
  (return (Utilities|Array|MakeArray Start (+ (Math|Vector|Lerp(Vector) Start End 0.25) "0.000000,0.000000,700.000000") (+ (Math|Vector|Lerp(Vector) Start End 0.5) "0.000000,0.000000,1000.000000") (+ (Math|Vector|Lerp(Vector) Start End 0.75) "0.000000,0.000000,700.000000") End)))