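; Mage projectile Blueprint that flies to a target and attacks the enemy it hits.
; Each tick calls FlyToTarget; overlapping a BP_BaseEnemy triggers AttackSingleEnemy on it, then destroys the bullet.
; MakeBezierPoints builds a five-point path from start to end, with randomized horizontal offsets and raised middle points for a varied arc.
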(event EventBeginPlay
  (|CallParentFunction) ; This node is disabled and will not be called.\nDrag off pins to build functionality.
)

(event Collision|EventActorBeginOverlap
  (params (OtherActor :type Actor%20Object%20Reference))
  (|CallParentFunction OtherActor)
  (bind _asbp_base_enemy (Utilities|Casting|CastToBP_BaseEnemy OtherActor))
  (CallFunction|AttackSingleEnemy _asbp_base_enemy)
  (Actor|DestroyActor))

(event EventTick
  (params (DeltaSeconds :type Float%20%28single-precision%29))
  (|CallParentFunction DeltaSeconds)
  (CallFunction|FlytoTarget))

(fn ConstructionScript
  (|CallParentFunction))

(fn MakeBezierPoints
  (params (Start :type Vector :default "0, 0, 0") (End :type Vector :default "0, 0, 0"))
  (bind _returnvalue (Math|Random|RandomFloatinRange -3e+02 3e+02))
  (return (Utilities|Array|MakeArray Start (+ (Math|Vector|Lerp(Vector) Start End 0.25) (Math|Vector|MakeVector _returnvalue _returnvalue 1e+02)) (+ (Math|Vector|Lerp(Vector) Start End 0.5) (Math|Vector|MakeVector _returnvalue _returnvalue 2e+02)) (+ (Math|Vector|Lerp(Vector) Start End 0.75) (Math|Vector|MakeVector _returnvalue _returnvalue 1e+02)) End)))