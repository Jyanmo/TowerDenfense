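; Archer projectile Blueprint that flies to a target and attacks a single enemy on hit, building on inherited bullet behavior.
; Tick calls FlyToTarget every frame, and overlapping a BP_BaseEnemy calls AttackSingleEnemy before destroying the projectile.
; MakeBezierPoints supplies five control points between start and end, raised along Z toward the midpoint to form an arched path.
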(event EventBeginPlay
  (|CallParentFunction))

(event Collision|EventActorBeginOverlap
  (params (OtherActor :type Actor%20Object%20Reference))
  (|CallParentFunction OtherActor)
  (bind _asbp_base_enemy (Utilities|Casting|CastToBP_BaseEnemy OtherActor))
  (CallFunction|AttackSingleEnemy _asbp_base_enemy)
  (Actor|DestroyActor))

(event EventTick
  (params (DeltaSeconds :type Float%20%28single-precision%29))
  (|CallParentFunction DeltaSeconds)
  (CallFunction|FlytoTarget))

(fn ConstructionScript
  (|CallParentFunction))

(fn MakeBezierPoints
  (params (Start :type Vector :default "0, 0, 0") (End :type Vector :default "0, 0, 0"))
  (return (Utilities|Array|MakeArray Start (+ (Math|Vector|Lerp(Vector) Start End 0.25) "0.000000,0.000000,100.000000") (+ (Math|Vector|Lerp(Vector) Start End 0.5) "0.000000,0.000000,200.000000") (+ (Math|Vector|Lerp(Vector) Start End 0.75) "0.000000,0.000000,100.000000") End)))