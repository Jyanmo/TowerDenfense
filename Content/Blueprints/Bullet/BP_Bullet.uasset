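; BP_Bullet is a base-style projectile that flies toward a target actor and provides a function to damage one enemy.
; BeginPlay derives flight time from distance and speed and requests Bezier points from MakeBezierPoints, an empty stub here.
; FlyToTarget follows a recursive De Casteljau curve, switches to homing velocity late in flight, faces its motion, and self-destroys without a target.
; Tick is empty, and nothing here calls the flight or attack functions.
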(event EventBeginPlay
  (Variables|/Script/Engine.ProjectileMovementComponent|SetInitialSpeed (Variables|Default|GetProjectileMovement) (Variables|Default|GetSpeed))
  (Variables|Default|SetTime (/ (Math|Vector|Distance(Vector) (Transformation|GetActorLocation) (Transformation|GetActorLocation (Variables|Default|GetTarget))) (Variables|Default|GetSpeed)))
  (Variables|Default|SetBezierPoints (CallFunction|MakeBezierPoints (Transformation|GetActorLocation) (Transformation|GetActorLocation (Variables|Default|GetTarget))))
  (Variables|Default|SetLastLoc (Transformation|GetActorLocation)))

(event EventTick
  (params (DeltaSeconds :type Float%20%28single-precision%29)))

(fn ConstructionScript)

(fn FlytoTarget
  (bind _returnvalue (Actor|GetGameTimeSinceCreation))
  (bind _time (Variables|Default|GetTime))
  (bind _returnvalue_2 (/ _returnvalue _time))
  (Utilities|IsValid (Variables|Default|GetTarget)
    (:Is%20Valid
      (Utilities|FlowControl|Sequence
        (:then_0
          (if (> _returnvalue_2 0.8)
            (Variables|/Script/Engine.MovementComponent|SetVelocity (Variables|Default|GetProjectileMovement) (* (Variables|Default|GetSpeed) (Math|Vector|Normalize (- (Transformation|GetActorLocation (Variables|Default|GetTarget)) (Transformation|GetActorLocation)))))
            (else
              (Transformation|SetActorLocation (CallFunction|Bezier (Variables|Default|GetBezierPoints) _returnvalue_2) false false))))
        (:then_1
          (Transformation|SetActorRotation (Math|Rotator|FindLookatRotation (Variables|Default|GetLastLoc) (Transformation|GetActorLocation)))
          (Variables|Default|SetLastLoc (Transformation|GetActorLocation)))))
    (:Is%20Not%20Valid
      (Actor|DestroyActor))))

(fn AttackSingleEnemy
  (params (Enemy :type BP%20Base%20Enemy%20Object%20Reference))
  (Class|BaseCharacter|LoseHealth Enemy (Variables|Default|GetDamage) (Variables|Default|GetDamageType))
  (Default|SetHealthBar Enemy))

(fn Bezier
  (params (Points :type Array%20of%20Vectors) (T :type Float%20%28double-precision%29))
  (if (== (Utilities|Array|Length Points) 1)
    (return (Utilities|Array|Get(acopy) Points))
    (else
      (for _index (range 0 (- (Utilities|Array|Length Points) 2))
        (Utilities|Array|Add (LocalVariables|GetRes) (Math|Vector|Lerp(Vector) (Utilities|Array|Get(acopy) Points _index) (Utilities|Array|Get(acopy) Points (+ _index 1)) T)))
      (return (CallFunction|Bezier (LocalVariables|GetRes) T)))))

(fn MakeBezierPoints
  (params (Start :type Vector) (End :type Vector))
  (return 0))

(fn FlytoLocation
  (Transformation|SetActorLocation (CallFunction|Bezier (Variables|Default|GetBezierPoints) (/ (Actor|GetGameTimeSinceCreation) (Variables|Default|GetTime))) false false))