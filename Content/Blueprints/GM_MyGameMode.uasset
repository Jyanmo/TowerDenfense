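; Game mode that starts an enemy wave along a spline path when play begins.
; BeginPlay caches the level's BP_Line actor, then spawns a BP_EnemyFactory and asks it to create a batch of Enemy_01 enemies on that line.
; A separate CreateEnemy function, not called within this graph, spawns one BP_BaseEnemy at the spline's first point with random horizontal jitter, handing it the line.
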(event EventBeginPlay
  (Utilities|FlowControl|Sequence
    (:then_0
      (bind _returnvalue (Actor|GetActorOfClass "/Game/Blueprints/BP_Line.BP_Line_C"))
      (Variables|Default|SetLine _returnvalue))
    (:then_1
      (bind _returnvalue_2 (Game|SpawnActorfromClass "/Game/Blueprints/BP_EnemyFactory.BP_EnemyFactory_C" (Math|Transform|MakeTransform "0, 0, 0") "Undefined" "MultiplyWithRoot" 0 0))
      (Default|CreateEnemyEvent _returnvalue_2 "Enemy_01" 10 (Variables|Default|GetLine)))))

(event EventTick
  (params (DeltaSeconds :type Float%20%28single-precision%29)))

(fn ConstructionScript)

(fn CreateEnemy
  (bind _line (Variables|Default|GetLine))
  (Game|SpawnActorfromClass "/Game/Characters/Enemy/Blueprints/BP_BaseEnemy.BP_BaseEnemy_C" (Math|Transform|MakeTransform (+ (Spline|GetLocationatSplinePoint (Variables|/Game/Blueprints/BP_Line.BP_Line_C|GetSpline _line) 0 "World") (Math|Vector|MakeVector (Math|Random|RandomFloatinRange -5e+01 5e+01) (Math|Random|RandomFloatinRange -5e+01 5e+01) 0.0)) "0, 0, 0" "1.000000,1.000000,1.000000") "AdjustIfPossibleButAlwaysSpawn" "MultiplyWithRoot" 0 _line 0))