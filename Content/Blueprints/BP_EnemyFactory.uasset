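; BP_EnemyFactory spawns waves of enemies at the start of a spline line, given a data table row name and a count.
; GetEnemyClass reads the BP_BaseEnemy class from DT_EnemyData, and each spawned enemy receives the line and initializes from that row.
; CreateEnemyEvent calls itself with a decremented count after a short delay, staggering spawns with slight random XY offsets around the first spline point.
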(event Custom|CreateEnemyEvent
  (params (EnemyRowName :type Name) (Count :type Integer) (Line :type BP%20Line%20Object%20Reference))
  (if (not (== Count 0))
    (bind _returnvalue (Game|SpawnActorfromClass (CallFunction|GetEnemyClass EnemyRowName) (Math|Transform|MakeTransform (CallFunction|RandomLocation Line) "0, 0, 0" "1.000000,1.000000,1.000000") "AdjustIfPossibleButAlwaysSpawn" "MultiplyWithRoot" 0 Line 0))
    (Class|BaseEnemy|Init _returnvalue EnemyRowName "/Game/DT/DT_EnemyData.DT_EnemyData")
    (Utilities|FlowControl|Delay 0.5)
    (CallFunction|CreateEnemyEvent EnemyRowName (- Count 1) Line)))

(event EventBeginPlay)

(event Collision|EventActorBeginOverlap
  (params (OtherActor :type Actor%20Object%20Reference)))

(event EventTick
  (params (DeltaSeconds :type Float%20%28single-precision%29)))

(fn ConstructionScript)

(fn GetEnemyClass
  (params (RowName :type Name))
  (bind _returnvalue (Utilities|GetDataTableRow "/Game/DT/DT_EnemyData.DT_EnemyData" RowName)
    (:then
      (bind _asbp_base_enemy (Utilities|Casting|CastToBP_BaseEnemyClass (.bpclass (.characterproperty _returnvalue))))
      (return _asbp_base_enemy))))

(fn RandomLocation
  (params (Line :type BP%20Line%20Object%20Reference))
  (return (+ (Spline|GetLocationatSplinePoint (Variables|/Game/Blueprints/BP_Line.BP_Line_C|GetSpline Line) 0 "World") (Math|Vector|MakeVector (Math|Random|RandomFloatinRange -5e+01 5e+01) (Math|Random|RandomFloatinRange -5e+01 5e+01) 0.0))))