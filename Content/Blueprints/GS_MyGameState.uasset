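; GS_MyGameState is a game state Blueprint that holds the game's coin count.
; AddCoins increases the stored count by a given amount.
; TryUseCoins deducts a requested amount and returns true, or returns false without spending when the request exceeds the balance.
; Event BeginPlay, Tick and the construction script are empty, so all logic lives in these two functions.
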(event EventBeginPlay)

(event EventTick
  (params (DeltaSeconds :type Float%20%28single-precision%29)))

(fn ConstructionScript)

(fn TryUseCoins
  (params (Coins :type Integer))
  (if (> Coins (Variables|Default|GetCoins))
    (return false)
    (else
      (Variables|Default|SetCoins (- (Variables|Default|GetCoins) Coins))
      (return true))))

(fn AddCoins
  (params (Coins :type Integer))
  (Variables|Default|SetCoins (+ Coins (Variables|Default|GetCoins))))