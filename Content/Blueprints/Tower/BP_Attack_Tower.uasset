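; Attack tower base that detects enemies in range and attacks on a cooldown, with Attack left as an empty stub.
; A looping timer refreshes Hits via sphere trace, and Tick calls Attack when targets exist, then starts the reload delay.
; AttackSingleEnemy spawns a bullet with random damage at an attackable enemy chosen by GetClosestEnemy, which compares a candidate's remaining distance against the current pick's walked distance.
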(event Custom|Reload
  (Utilities|FlowControl|Delay (Class|BaseTower|GetAttackCoolDownTime))
  (Variables|Default|SetbCanAttack true))

(event EventBeginPlay
  (|CallParentFunction)
  (Utilities|Time|SetTimerbyFunctionName 0 "Detect" 0.5 true))

(event Collision|EventActorBeginOverlap
  (params (OtherActor :type Actor%20Object%20Reference))
  (|CallParentFunction OtherActor) ; This node is disabled and will not be called.\nDrag off pins to build functionality.
)

(event EventTick
  (params (DeltaSeconds :type Float%20%28single-precision%29))
  (|CallParentFunction DeltaSeconds)
  (if (and (Utilities|Array|IsNotEmpty (Variables|Default|GetHits)) (Variables|Default|GetbCanAttack))
    (CallFunction|Attack)
    (Variables|Default|SetbCanAttack false)
    (CallFunction|Reload)))

(fn ConstructionScript
  (|CallParentFunction))

(fn Detect
  (bind _returnvalue (Transformation|GetActorLocation))
  (bind _outhits (Collision|MultiSphereTraceForObjects _returnvalue _returnvalue (Math|Conversions|ToFloat(Integer) (Class|BaseTower|GetAttackRange)) (Utilities|Array|MakeArray "ObjectTypeQuery7") false 0 "None"))
  (Variables|Default|SetHits _outhits))

(fn Attack)

(fn AttackSingleEnemy
  (bind _hits (Variables|Default|GetHits))
  (bind (_resenemy _ressult) (CallFunction|GetClosestEnemy _hits))
  (if _ressult
    (Game|SpawnActorfromClass "/Game/Blueprints/Bullet/BP_Bullet.BP_Bullet_C" (Math|Conversions|ToTransform(Vector) (Transformation|GetWorldLocation (Variables|Default|GetFirePoint))) "AlwaysSpawn" "MultiplyWithRoot" 0 _resenemy (Class|BaseTower|GetProJectileSpeed) (Class|BaseTower|RandomDamage) 0)))

(fn GetClosestEnemy
  (params (Hits :type Array%20of%20Hit%20Result%20Structures))
  (for _array_element Hits
    (bind _asbp_base_enemy (Utilities|Casting|CastToBP_BaseEnemy (.HitActor (Collision|BreakHitResult _array_element))))
    (if (Class|BaseTower|IsEnemyAttackable _asbp_base_enemy)
      (Utilities|IsValid (LocalVariables|GetRes)
        (:Is%20Valid
          (if (< (Default|GetRemainDis _asbp_base_enemy) (Default|GetWalkedDis (LocalVariables|GetRes)))
            (LocalVariables|SetRes _asbp_base_enemy)))
        (:Is%20Not%20Valid
          (LocalVariables|SetRes _asbp_base_enemy)))))
  (Utilities|IsValid (LocalVariables|GetRes)
    (:Is%20Valid
      (return (LocalVariables|GetRes) true))
    (:Is%20Not%20Valid
      (return 0 true))))