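; Base tower actor that is set up from a DT_TowerData row and can be upgraded or sold.
; Initialize applies the row's meshes and first cost and hides its TowerLand plot; LevelUp sets Value to the next cost, increments Level and refreshes meshes.
; Clicking it opens and resets the HUD build panel for this tower.
; Sell refunds 60% of Value through the GameState, re-shows the plot and destroys the tower.
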(event EventBeginPlay
  (bind _asgm_my_game_mode (Utilities|Casting|CastToGM_MyGameMode (Game|GetGameMode)))
  (Variables|Default|SetGameMode _asgm_my_game_mode)
  (bind _asgs_my_game_state (Utilities|Casting|CastToGS_MyGameState (Game|GetGameState)))
  (Variables|Default|SetGameState _asgs_my_game_state))

(event Collision|EventActorBeginOverlap
  (params (OtherActor :type Actor%20Object%20Reference)))

(event EventTick
  (params (DeltaSeconds :type Float%20%28single-precision%29)))

(event MouseInput|EventActorOnClicked
  (params (ButtonPressed :type Key%20Structure :default "None"))
  (bind _gamemode (Variables|Default|GetGameMode))
  (bind _hud (Variables|/Game/Blueprints/GM_MyGameMode.GM_MyGameMode_C|GetHUD _gamemode))
  (Default|ShowBulidPanel _hud (Transformation|GetActorLocation))
  (Default|Reset (Variables|/Game/UI/WBP_GameHUD.WBP_GameHUD_C|GetWBP_BulidPanel _hud) self))

(fn ConstructionScript)

(fn Initialize
  (params (RowName :type Name))
  (Utilities|FlowControl|Sequence
    (:then_0
      (Class|BaseTower|Init RowName "/Game/DT/DT_TowerData.DT_TowerData")
      (CallFunction|SetMesh)
      (bind _returnvalue (Utilities|GetDataTableRow "/Game/DT/DT_TowerData.DT_TowerData" RowName)
        (:then
          (Variables|Default|SetValue (Utilities|Array|Get(acopy) (.cost _returnvalue))))))
    (:then_1
      (Rendering|SetVisibility (Variables|/Game/Blueprints/Tower/BP_TowerLand.BP_TowerLand_C|GetDefaultSceneRoot (Variables|Default|GetTowerLand)) false true))))

(fn SetMesh
  (Components|StaticMesh|SetStaticMesh (Variables|Default|GetStaticMesh) (Class|BaseTower|GetStaticMesh))
  (Components|SkeletalMesh|SetSkeletalMeshAsset (Variables|Default|GetSkeletalMesh) (Class|BaseTower|GetSkeletalMesh)))

(fn LevelUp
  (Variables|Default|SetValue (Class|BaseTower|GetNextCost))
  (Math|Integer|IncrementInt (Variables|Default|GetLevel)
    (:%20%20
      (CallFunction|SetMesh))))

(fn Sell
  (Default|AddCoins (Variables|Default|GetGameState) (Math|Float|Truncate (* (Variables|Default|GetValue) 0.6)))
  (Rendering|SetVisibility (Variables|/Game/Blueprints/Tower/BP_TowerLand.BP_TowerLand_C|GetDefaultSceneRoot (Variables|Default|GetTowerLand)) true true)
  (Actor|DestroyActor))