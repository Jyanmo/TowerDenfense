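; BP_TowerLand is a clickable tower plot that opens the HUD build panel at its location.
; On click it resets the panel for itself and registers as the GameMode's current tower land.
; It then binds to the player controller's left-click event, so the next click collapses the panel and unbinds.
; One-tick delays precede showing the panel and binding that event.
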(event Custom|CustomEvent
  (Widget|SetVisibility (Variables|/Game/UI/WBP_GameHUD.WBP_GameHUD_C|GetWBP_BulidPanel (Variables|/Game/Blueprints/GM_MyGameMode.GM_MyGameMode_C|GetHUD (Variables|Default|GetGameMode))) "Collapsed")
  (EventDispatchers|UnbindEventfromOnLeftMouseClicked (stale MouseInput|EventActorOnClicked _aspc_my_player_controller) (delegate Custom|CustomEvent)))

(event EventBeginPlay
  (bind _asgm_my_game_mode (Utilities|Casting|CastToGM_MyGameMode (Game|GetGameMode)))
  (Variables|Default|SetGameMode _asgm_my_game_mode))

(event Collision|EventActorBeginOverlap
  (params (OtherActor :type Actor%20Object%20Reference)))

(event EventTick
  (params (DeltaSeconds :type Float%20%28single-precision%29)))

(event MouseInput|EventActorOnClicked
  (params (ButtonPressed :type Key%20Structure :default "None"))
  (bind _gamemode (Variables|Default|GetGameMode))
  (bind _hud (Variables|/Game/Blueprints/GM_MyGameMode.GM_MyGameMode_C|GetHUD _gamemode))
  (Utilities|FlowControl|DelayUntilNextTick)
  (Default|ShowBulidPanel _hud (Transformation|GetActorLocation))
  (Default|Reset (Variables|/Game/UI/WBP_GameHUD.WBP_GameHUD_C|GetWBP_BulidPanel _hud) self)
  (Variables|/Game/Blueprints/GM_MyGameMode.GM_MyGameMode_C|SetCurrentTowerLand _gamemode self)
  (bind _aspc_my_player_controller (Utilities|Casting|CastToPC_MyPlayerController (Game|GetPlayerController 0)))
  (Utilities|FlowControl|DelayUntilNextTick)
  (EventDispatchers|BindEventtoOnLeftMouseClicked _aspc_my_player_controller (delegate Custom|CustomEvent)))

(fn ConstructionScript)