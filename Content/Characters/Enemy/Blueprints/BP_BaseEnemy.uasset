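; BP_BaseEnemy is a base enemy Blueprint positioned relative to a spline on its Line reference.
; Its construction script stores Distance as the signed offset from the nearest spline point, with the sign taken from a side vector built from the first point's tangent crossed with world down.
; GetWalkedDis returns the distance along the spline at the point closest to the enemy.
; The event graph holds no active logic.
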(event EventBeginPlay)

(event Collision|EventActorBeginOverlap
  (params (OtherActor :type Actor%20Object%20Reference)))

(event EventTick
  (params (DeltaSeconds :type Float%20%28single-precision%29)))

(fn ConstructionScript
  (bind _returnvalue (Transformation|GetActorLocation))
  (bind _line (Variables|Default|GetLine))
  (bind _spline (Variables|/Game/Blueprints/BP_Line.BP_Line_C|GetSpline _line))
  (bind _returnvalue_2 (Spline|FindLocationClosesttoWorldLocation _spline _returnvalue "World"))
  (bind _returnvalue_3 (- _returnvalue _returnvalue_2))
  (bind _returnvalue_4 (Math|Vector|VectorLength _returnvalue_3))
  (if (> (Math|Vector|DotProduct _returnvalue_3 (Math|Vector|Normalize (Math|Vector|CrossProduct (Spline|GetTangentatSplinePoint _spline 0 "World") "0.000000,0.000000,-1.000000"))) 0.0)
    (Variables|Default|SetDistance _returnvalue_4)
    (else
      (Variables|Default|SetDistance (* _returnvalue_4 -1.0)))))

(fn GetWalkedDis
  (bind _line (Variables|Default|GetLine))
  (bind _spline (Variables|/Game/Blueprints/BP_Line.BP_Line_C|GetSpline _line))
  (return (Class|SplineComponent|GetDistanceAlongSplineatSplineInputKey _spline (Class|SplineComponent|FindInputKeyClosesttoWorldLocation _spline (Transformation|GetActorLocation)))))