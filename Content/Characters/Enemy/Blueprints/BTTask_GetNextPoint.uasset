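; Behavior tree task that gives an enemy its next point along its assigned spline line.
; It samples the BP_BaseEnemy's spline a fixed distance ahead of its walked distance.
; It offsets that point sideways by the enemy's Distance value, crossing the spline tangent with the down vector to get the perpendicular.
; The result is written to the selected blackboard key and the task finishes successfully.
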(event EventReceiveExecuteAI
  (params (OwnerController :type AI%20Controller%20Object%20Reference) (ControlledPawn :type Pawn%20Object%20Reference))
  (bind _asbp_base_enemy (Utilities|Casting|CastToBP_BaseEnemy ControlledPawn))
  (AI|BehaviorTree|SetBlackboardValueasVector (Variables|Default|GetSelector) (+ (Spline|GetLocationatDistanceAlongSpline (Variables|/Game/Blueprints/BP_Line.BP_Line_C|GetSpline (Variables|/Game/Characters/Enemy/Blueprints/BP_BaseEnemy.BP_BaseEnemy_C|GetLine _asbp_base_enemy)) (+ (Default|GetWalkedDis _asbp_base_enemy) 5e+02) "World") (* (Math|Vector|Normalize (Math|Vector|CrossProduct (Spline|GetTangentatDistanceAlongSpline (Variables|/Game/Blueprints/BP_Line.BP_Line_C|GetSpline (Variables|/Game/Characters/Enemy/Blueprints/BP_BaseEnemy.BP_BaseEnemy_C|GetLine _asbp_base_enemy)) (+ (Default|GetWalkedDis _asbp_base_enemy) 5e+02) "World") "0.000000,0.000000,-1.000000")) (Variables|/Game/Characters/Enemy/Blueprints/BP_BaseEnemy.BP_BaseEnemy_C|GetDistance _asbp_base_enemy))))
  (AI|BehaviorTree|FinishExecute true))